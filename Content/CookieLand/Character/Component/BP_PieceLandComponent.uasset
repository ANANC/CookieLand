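; Character component that moves a player across the pieces of a CookieLand board and shows the win panel at the finish.
; Initial placement caches walk speed and snaps the character to the piece, offset by capsule half-height.
; Later steps, except Up or Down, send a move action targeting CurPieceId to MoveToComponent.
; That move runs at full speed beyond roughly one piece interval, otherwise at reduced speed.
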(event EventMovetoInitialLocation
  (params (pieceId :type Integer) (location :type Vector :default "0, 0, 0"))
  (if (== (Variables|Default|GetPlayerMaxSpeed) 0.0)
    (Variables|Default|SetPlayerMaxSpeed (Variables|/Script/Engine.CharacterMovementComponent|GetMaxWalkSpeed (Class|BaseCharacter|GetCharacterMovementComponent (Variables|Default|GetCharacter)))))
  (CallFunction|UpdateCharacterLocation pieceId location "Left" true))

(event EventMovetoNextLocation
  (params (pieceId :type Integer) (location :type Vector :default "0, 0, 0") (moveDirection :type EPieceDirection%20Enum :default "Left"))
  (CallFunction|UpdateCharacterLocation pieceId location moveDirection false))

(event EventStandbyFinishLocation
  (bind _returnvalue (UserInterface|CreateWidget "/Game/CookieLand/UI/WBP_WinPanel.WBP_WinPanel_C" (Game|GetPlayerController 0)))
  (UserInterface|Viewport|AddtoPlayerScreen _returnvalue 1))

(fn UpdateCharacterLocation
  (params (pieceId :type Integer) (location :type Vector) (moveDirection :type EPieceDirection%20Enum :default "Left") (isForceUpdate :type Boolean))
  (Variables|Default|SetTargetLocation (+ location (Math|Vector|MakeVector 0.0 0.0 (+ (Variables|/Script/Engine.CapsuleComponent|GetCapsuleHalfHeight (Variables|/Script/Engine.Character|GetCapsuleComponent (Variables|Default|GetCharacter))) 0.0))))
  (if isForceUpdate
    (Transformation|SetActorLocation (Variables|Default|GetCharacter) (Variables|Default|GetTargetLocation) false false)
    (elif (and (Utilities|Enum|NotEqual(Enum) moveDirection "Up") (Utilities|Enum|NotEqual(Enum) moveDirection "Down"))
      (Utilities|FlowControl|Sequence
        (:then_0
          (bind _returnvalue (Game|ConstructObjectfromClass "/Script/CookieLand.AIReactionMoveToPieceActionData"))
          (bind _output_get (LocalVariables|SetMoveToPieceAction _returnvalue))
          (Variables|/Script/CookieLand.AIReactionMoveToPieceActionData|SetTargetPieceId _output_get (Variables|Default|GetCurPieceId))
          (Variables|/Script/CookieLand.AIReactionBaseMoveToActionData|SetAcceptance _output_get 1e+01)
          (Variables|/Script/CookieLand.AIReactionBaseMoveToActionData|SetShowDebugLine _output_get false)
          (if (> (Math|Vector|Distance2D(Vector) (Transformation|GetActorLocation (Variables|Default|GetCharacter)) (Variables|Default|GetTargetLocation)) (+ (.x (Variables|/Script/CookieLand.LandDataAsset|GetActorInterval (Variables|/Script/CookieLand.BasePieceLand|GetLandDataAsset (Class|CommonFunctionLibrary|GetCurPieceLand)))) 5e+01))
            (Variables|/Script/CookieLand.AIReactionBaseMoveToActionData|SetFixedSpeed _returnvalue (Variables|Default|GetPlayerMaxSpeed))
            (else
              (Variables|/Script/CookieLand.AIReactionBaseMoveToActionData|SetFixedSpeed _output_get (* (Variables|Default|GetPlayerMaxSpeed) 0.6)))))
        (:then_1
          (Class|MovetoComponent|Moveto (Variables|/Script/CookieLand.BaseCharacter|GetMoveToComponent (Variables|Default|GetCharacter)) (LocalVariables|GetMoveToPieceAction)))))))