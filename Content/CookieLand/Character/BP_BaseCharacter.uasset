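; BP_BaseCharacter is a player-controlled character for CookieLand that supports both board-piece movement and free movement with jumping.
; On possession it adds its Enhanced Input mapping context, then applies the stored Yaw on the next tick.
; Board inputs, gated by EnableControlInputInfo, become character-relative land directions for PieceLandComponent, while free inputs use AddMovementInput.
; Other inputs rotate control yaw in 90-degree steps, adjust spring-arm length and toggle a debug menu.
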(event Custom|CustomEvent
  (Transformation|SetActorRotation (Math|Rotator|MakeRotator 0.0 0.0 (Variables|Default|GetYaw)))
  (Pawn|SetControlRotation (Pawn|GetController) (Math|Rotator|MakeRotator 0.0 0.0 (Variables|Default|GetYaw))))

(event Input|EnhancedActionEvents|EnhancedInputActionTurn90LRCC1
  (params (ActionValue :type Float%20%28double-precision%29) (ElapsedSeconds :type Float%20%28double-precision%29) (TriggeredSeconds :type Float%20%28double-precision%29) (InputAction :type Input%20Action%20Object%20Reference :default "/Game/CookieLand/Character/Input/Turn90LRCC1.Turn90LRCC1"))
  (CallFunction|RotationController ActionValue))

(event Input|EnhancedActionEvents|EnhancedInputActionTurnLRCC
  (params (ActionValue :type Float%20%28double-precision%29) (ElapsedSeconds :type Float%20%28double-precision%29) (TriggeredSeconds :type Float%20%28double-precision%29) (InputAction :type Input%20Action%20Object%20Reference :default "/Game/CookieLand/Character/Input/TurnLRCC.TurnLRCC")))

(event Input|EnhancedActionEvents|EnhancedInputActionTurnUDCC
  (params (ActionValue :type Float%20%28double-precision%29) (ElapsedSeconds :type Float%20%28double-precision%29) (TriggeredSeconds :type Float%20%28double-precision%29) (InputAction :type Input%20Action%20Object%20Reference :default "/Game/CookieLand/Character/Input/TurnUDCC.TurnUDCC")))

(event Input|EnhancedActionEvents|EnhancedInputActionMoveToForwardCC
  (params (ActionValue :type Boolean) (ElapsedSeconds :type Float%20%28double-precision%29) (TriggeredSeconds :type Float%20%28double-precision%29) (InputAction :type Input%20Action%20Object%20Reference :default "/Game/CookieLand/Character/Input/MoveToForwardCC.MoveToForwardCC"))
  ;[1 1 1] 棋盘移动模式
  (if (== ActionValue true)
    (CallFunction|InputMovetoNextPiece "Forward")
    (else
      (CallFunction|InputMovetoNextPiece "Backward"))))

(event Input|EnhancedActionEvents|EnhancedInputActionMoveToRightCC
  (params (ActionValue :type Boolean) (ElapsedSeconds :type Float%20%28double-precision%29) (TriggeredSeconds :type Float%20%28double-precision%29) (InputAction :type Input%20Action%20Object%20Reference :default "/Game/CookieLand/Character/Input/MoveToRightCC.MoveToRightCC"))
  ;[1 1 1] 棋盘移动模式
  (if (== ActionValue true)
    (CallFunction|InputMovetoNextPiece "Right")
    (else
      (CallFunction|InputMovetoNextPiece "Left"))))

(event Input|EnhancedActionEvents|EnhancedInputActionMoveToForwardFreeCC
  (params (ActionValue :type Float%20%28double-precision%29) (ElapsedSeconds :type Float%20%28double-precision%29) (TriggeredSeconds :type Float%20%28double-precision%29) (InputAction :type Input%20Action%20Object%20Reference :default "/Game/CookieLand/Character/Input/MoveToForwardFreeCC.MoveToForwardFreeCC"))
  ;[1 1 1] 自由移动模式
  (Pawn|Input|AddMovementInput (Math|Vector|GetForwardVector (Transformation|GetActorRotation)) ActionValue false))

(event Input|EnhancedActionEvents|EnhancedInputActionMoveToRightFreeCC
  (params (ActionValue :type Float%20%28double-precision%29) (ElapsedSeconds :type Float%20%28double-precision%29) (TriggeredSeconds :type Float%20%28double-precision%29) (InputAction :type Input%20Action%20Object%20Reference :default "/Game/CookieLand/Character/Input/MoveToRightFreeCC.MoveToRightFreeCC"))
  ;[1 1 1] 自由移动模式
  (Pawn|Input|AddMovementInput (Math|Vector|GetRightVector (Transformation|GetActorRotation)) ActionValue false))

(event Input|EnhancedActionEvents|EnhancedInputActionJumpCC
  (params (ActionValue :type Boolean) (ElapsedSeconds :type Float%20%28double-precision%29) (TriggeredSeconds :type Float%20%28double-precision%29) (InputAction :type Input%20Action%20Object%20Reference :default "/Game/CookieLand/Character/Input/JumpCC.JumpCC"))
  ;[1 1 1] 自由移动模式
  (Character|Jump))

(event Input|EnhancedActionEvents|EnhancedInputActionCameraTargetArmLengthCC
  (params (ActionValue :type Float%20%28double-precision%29) (ElapsedSeconds :type Float%20%28double-precision%29) (TriggeredSeconds :type Float%20%28double-precision%29) (InputAction :type Input%20Action%20Object%20Reference :default "/Game/CookieLand/Character/Input/CameraTargetArmLengthCC.CameraTargetArmLengthCC"))
  (bind _springarm (Variables|Default|GetSpringArm))
  ;[1 1 1] 相机事件
  (Variables|/Script/Engine.SpringArmComponent|SetTargetArmLength _springarm (+ (* ActionValue 1e+02) (Variables|/Script/Engine.SpringArmComponent|GetTargetArmLength _springarm))))

(event Input|EnhancedActionEvents|EnhancedInputActionOpenDebugMenuCC
  (params (ActionValue :type Boolean) (ElapsedSeconds :type Float%20%28double-precision%29) (TriggeredSeconds :type Float%20%28double-precision%29) (InputAction :type Input%20Action%20Object%20Reference :default "/Game/CookieLand/Character/Input/OpenDebugMenuCC.OpenDebugMenuCC"))
  (bind _output_get (Variables|Default|SetIsOpeningDebugMenu (not (Variables|Default|GetIsOpeningDebugMenu))))
  (if _output_get
    (bind _returnvalue (UserInterface|CreateWidget "/Game/CookieLand/UI/WBP_DebugMenu.WBP_DebugMenu_C" (Game|GetPlayerController 0)))
    (bind _output_get_2 (Variables|Default|SetDebugMenuWidget _returnvalue))
    (UserInterface|Viewport|AddtoPlayerScreen _output_get_2)
    (else
      (Utilities|IsValid (Variables|Default|GetDebugMenuWidget)
        (:Is%20Valid
          (Widget|RemovefromParent (Variables|Default|GetDebugMenuWidget)))))))

(event EventBeginPlay)

(event Collision|EventActorBeginOverlap
  (params (OtherActor :type Actor%20Object%20Reference)))

(event EventPossessed
  (params (NewController :type Controller%20Object%20Reference))
  (bind _asplayer_controller (Utilities|Casting|CastToPlayerController NewController))
  (Input|AddMappingContext (PlayerController|LocalPlayerSubsystems|GetEnhancedInputLocalPlayerSubsystem _asplayer_controller) "/Game/CookieLand/Character/Input/IM_CharacterCC.IM_CharacterCC" 0 "(bIgnoreAllPressedKeysUntilRelease=True,bForceImmediately=False,bNotifyUserSettings=False)")
  (Class|KismetSystemLibrary|SetTimerforNextTickDelegate (delegate Custom|CustomEvent)))

(fn ConstructionScript)

(fn CanJumpInternal
  (return true))

(fn SetEnableControlInputInfo
  (params (enable :type Boolean))
  (Variables|Default|SetEnableControlInputInfo enable))

(fn InputMovetoNextPiece
  (params (Dir :type EPieceDirection%20Enum :default "Left"))
  (if (Variables|Default|GetEnableControlInputInfo)
    (switch Utilities|FlowControl|Switch|SwitchonEPieceDirection Dir
      (:Left
        (Class|PieceLandComponent|MovetoNextPiece (Variables|Default|GetPieceLandComponent) (Class|CommonFunctionLibrary|ChangetoLandDirectionbyCharacter "Left" self)))
      (:Right
        (Class|PieceLandComponent|MovetoNextPiece (Variables|Default|GetPieceLandComponent) (Class|CommonFunctionLibrary|ChangetoLandDirectionbyCharacter "Right" self)))
      (:Forward
        (Class|PieceLandComponent|MovetoNextPiece (Variables|Default|GetPieceLandComponent) (Class|CommonFunctionLibrary|ChangetoLandDirectionbyCharacter "Forward" self)))
      (:Backward
        (Class|PieceLandComponent|MovetoNextPiece (Variables|Default|GetPieceLandComponent) (Class|CommonFunctionLibrary|ChangetoLandDirectionbyCharacter "Backward" self))))))

(fn RotationController
  (params (direction :type Float%20%28double-precision%29))
  (bind _returnvalue (Pawn|GetController))
  (bind _returnvalue_2 (Transformation|GetActorRotation _returnvalue))
  (bind _output_get (Variables|Default|SetYaw (+ (* direction 9e+01) (Variables|Default|GetYaw))))
  (Pawn|SetControlRotation _returnvalue (Math|Rotator|MakeRotator (.roll _returnvalue_2) (.pitch _returnvalue_2) _output_get))
  (Default|CallUpdateControllerYaw))