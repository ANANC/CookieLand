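; BP_BasePiece is the base piece Blueprint in CookieLand, displaying a piece's movement rules through a text label and four directional landmark components.
; InitArt calls UpdatePieceArt, which reads enabled directions and distance from Piece.
; NumberText shows "Up" and/or "Down" when those moves are enabled, plus any distance limit in parentheses.
; Left, right, forward and backward landmarks are hidden when their direction is enabled, so visible ones mark disabled moves.
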(event EventBeginPlay)

(event Collision|EventActorBeginOverlap
  (params (OtherActor :type Actor%20Object%20Reference)))

(event EventInitArt
  (CallFunction|UpdatePieceArt))

(fn ConstructionScript)

(fn UpdatePieceArt
  (CallFunction|UpdateMoveDirection)
  (CallFunction|UpdateFourDLandmark))

(fn UpdateMoveDirection
  (if (or (Class|BasePiece|GetEnableMove (Variables|Default|GetPiece) "Up") (Class|BasePiece|GetEnableMove (Variables|Default|GetPiece) "Down"))
    (CallFunction|UpdateUporDownText)
    (else
      (CallFunction|UpdateFourDText))))

(fn UpdateUporDownText
  (bind _piece (Variables|Default|GetPiece))
  (bind _returnvalue (Class|BasePiece|GetCurInfo _piece))
  (bind _info (Variables|/Script/CookieLand.PieceInfo|GetInfo _returnvalue))
  (bind _distance (Variables|/Script/CookieLand.PieceBaseInfo|GetDistance _info))
  (Utilities|FlowControl|Sequence
    (:then_0
      (if (Class|BasePiece|GetEnableMove (Variables|Default|GetPiece) "Up")
        (LocalVariables|SetText (Utilities|String|Append (LocalVariables|GetText) "Up"))))
    (:then_1
      (if (Class|BasePiece|GetEnableMove (Variables|Default|GetPiece) "Down")
        (LocalVariables|SetText (Utilities|String|Append (LocalVariables|GetText) "Down"))))
    (:then_2
      (if (not (.isunlimit _distance))
        (LocalVariables|SetText (Utilities|String|Append (LocalVariables|GetText) "\\n" "(" (Utilities|String|ToString(Integer) (.limitdistance _distance)) ")"))))
    (:then_3
      (Rendering|Components|TextRender|SetText (Variables|Default|GetNumberText) (Utilities|Text|ToText(String) (LocalVariables|GetText))))))

(fn UpdateFourDText
  (bind _piece (Variables|Default|GetPiece))
  (bind _returnvalue (Class|BasePiece|GetCurInfo _piece))
  (bind _info (Variables|/Script/CookieLand.PieceInfo|GetInfo _returnvalue))
  (bind _distance (Variables|/Script/CookieLand.PieceBaseInfo|GetDistance _info))
  (Utilities|FlowControl|Sequence
    (:then_0
      (if (not (.isunlimit _distance))
        (LocalVariables|SetText (Utilities|String|Append (LocalVariables|GetText) "\\n" "(" (Utilities|String|ToString(Integer) (.limitdistance _distance)) ")"))))
    (:then_1
      (Rendering|Components|TextRender|SetText (Variables|Default|GetNumberText) (Utilities|Text|ToText(String) (LocalVariables|GetText))))))

(fn UpdateFourDLandmark
  (Utilities|FlowControl|Sequence
    (:then_0
      (Development|SetHiddeninGame (Variables|Default|GetLeftLandmark) (Class|BasePiece|GetEnableMove (Variables|Default|GetPiece) "Left") false))
    (:then_1
      (Development|SetHiddeninGame (Variables|Default|GetRightLandmark) (Class|BasePiece|GetEnableMove (Variables|Default|GetPiece) "Right") false))
    (:then_2
      (Development|SetHiddeninGame (Variables|Default|GetForwardLandmark) (Class|BasePiece|GetEnableMove (Variables|Default|GetPiece) "Forward") false))
    (:then_3
      (Development|SetHiddeninGame (Variables|Default|GetBackwardLandmark) (Class|BasePiece|GetEnableMove (Variables|Default|GetPiece) "Backward") false))))